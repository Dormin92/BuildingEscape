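; Openable door actor that swings open and closed when its OpenDoor member fires OnOpen and OnClose.
; BeginPlay caches the starting rotation and location.
; The DoorSwing timeline adds its OpenAngle yaw to that rotation, playing forward to open and reversing to close.
; An event track on the timeline plays the door sound at the cached location.
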(event OnOpen(OpenDoor)
  (bind _open_angle (Timeline|Door%20Swing Play)
    (:Update
      (Transformation|SetActorRotation (Math|Rotator|CombineRotators (Math|Rotator|MakeRotator 0.0 0.0 _open_angle) (Variables|Default|GetInitial%20Rotation))))
    (:Door%20Sound
      (Audio|PlaySoundatLocation "/Game/Audio/Door_Open.Door_Open" (Variables|Default|GetDoor%20Location) "0, 0, 0" 1.0 1.0 0.0 0 0 0))))

(event OnClose(OpenDoor)
  (bind _open_angle (Timeline|Door%20Swing Reverse)
    (:Update
      (Transformation|SetActorRotation (Math|Rotator|CombineRotators (Math|Rotator|MakeRotator 0.0 0.0 _open_angle) (Variables|Default|GetInitial%20Rotation))))
    (:Door%20Sound
      (Audio|PlaySoundatLocation "/Game/Audio/Door_Open.Door_Open" (Variables|Default|GetDoor%20Location) "0, 0, 0" 1.0 1.0 0.0 0 0 0))))

(event EventBeginPlay
  (Variables|Default|SetInitial%20Rotation (Transformation|GetActorRotation))
  (Variables|Default|SetDoor%20Location (Transformation|GetActorLocation)))

(fn ConstructionScript)